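; Player controller for a swipe-card city game in which the player accepts or declines laws.
; It pulls laws from the ResourceManager and shows them on the Bonanza HUD, locking input during card transitions.
; Paired MultiGates require two swipes in one direction: the first previews, the second commits, and switching direction resets the other.
; ResourceManager end events show a Polish summary card, where either confirmed swipe fades music and opens the main menu.
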(event `All Resources Full_Event_0`
  (set `self.Is Menu Enabled` true)
  (`KismetSystemLibrary.Delay` 0.7)
  (`self.Display Summary` "Świetnie!" "Miasto odżyło! \n \nPrzejść do kolejnego?"))

(event `All Resources Lost_Event_0`
  (set `self.Is Menu Enabled` true)
  (`KismetSystemLibrary.Delay` 0.7)
  (`self.Display Summary` "Oj..." "Coś nie pykło tutaj. \n \nKolejne miasto?"))

(event `All Laws Processed_Event_0`
  (set `self.Is Menu Enabled` true)
  (bind (_people_level _money_level _eco_level) (`/Game/ResourceManager/ResourceManager.Get City Stats` (`self.ResourceManager`)))
  (switch `int` (`KismetArrayLibrary.Array_Find` (`|MakeArray` _people_level _money_level _eco_level) (`KismetMathLibrary.Max` _people_level _money_level _eco_level))
    (:`Default`
      (`self.Display Summary` "Dobra robota" "Jedziemy dalej. \n \nKolejne miasto?"))
    (:`0`
      (`self.Display Summary` "Dobra robota" "Najważniesi są ludzie... bo to oni płacą podatki. \n \nKolejne miasto?"))
    (:`1`
      (`self.Display Summary` "Dobra robota" "W skarbcu mamy więcej złotych monet niż u samego McKwacza. \n \nKolejne miasto?"))
    (:`2`
      (`self.Display Summary` "Dobra robota" "Bida z nędzą, ale wczasy pod gruszą. \n \nKolejne miasto?"))))

(event `self.ReceiveBeginPlay`
  (`|ExecutionSequence`
    (:`then_0`
      (add `/Game/ResourceManager/ResourceManager.All Resources Full` (`self.ResourceManager`) (delegate `All Resources Full_Event_0`))
      (add `/Game/ResourceManager/ResourceManager.All Resources Lost` (`self.ResourceManager`) (delegate `All Resources Lost_Event_0`))
      (add `/Game/ResourceManager/ResourceManager.All Laws Processed` (`self.ResourceManager`) (delegate `All Laws Processed_Event_0`)))
    (:`then_1`
      (bind _returnvalue (`|CreateWidget` "/Game/UI/Bonanza_HUD.Bonanza_HUD_C" self))
      (bind _output_get (set `self.Bonanza HUD` _returnvalue))
      (`UserWidget.AddToViewport` _output_get 0)
      (`UserWidget.AddToViewport` _returnvalue 0))
    (:`then_2`
      (`self.DisableInput` self)
      (`KismetSystemLibrary.Delay` 2.0)
      (`self.Display Next Law`)
      (`/Game/UI/Bonanza_HUD.New Law Animation` (`self.Bonanza HUD`))
      (`KismetSystemLibrary.Delay` 0.5)
      (`self.EnableInput` self))
    (:`then_3`
      (`AudioComponent.FadeIn` (`self.Gameplay Music`) 3.0 1.0 0.0 "Linear"))))

(event `InputAction|Swipe Left`
  (params (Key :type "Key Structure"))
  (bind _resourcemanager (`self.ResourceManager`))
  (bind _bonanza_hud (`self.Bonanza HUD`))
  (bind _bonanza_hud_2 (`self.Bonanza HUD`))
  (bind _current_law_name (`self.Current Law Name`))
  ;[1 1 1] Input Swipe
  (:`Pressed`
    (if (`self.Is Menu Enabled`)
      (`self.Input Swipe Left Menu`)
      (else
        (`|MultiGate` false true :!label _label
          (:`Out 0`
            (`/Game/ResourceManager/ResourceManager.Try To Decline Law` _resourcemanager _current_law_name)
            (`/Game/UI/Bonanza_HUD.Try To Decline Animation` _bonanza_hud true)
            (goto _label_2 :!via `Reset`))
          (:`Out 1`
            (`/Game/ResourceManager/ResourceManager.Decline Law` _resourcemanager _current_law_name)
            (`self.DisableInput` self)
            (`/Game/UI/Bonanza_HUD.Decline Animation` _bonanza_hud)
            (`KismetSystemLibrary.Delay` 1.0)
            (`self.Display Next Law`)
            (`/Game/UI/Bonanza_HUD.New Law Animation` (`self.Bonanza HUD`))
            (`KismetSystemLibrary.Delay` 0.5)
            (`self.EnableInput` self)))))))

(event `InputAction|Swipe Right`
  (params (Key :type "Key Structure"))
  (bind _resourcemanager (`self.ResourceManager`))
  (bind _bonanza_hud (`self.Bonanza HUD`))
  (bind _current_law_name (`self.Current Law Name`))
  ;[1 1 1] Input Swipe
  (:`Pressed`
    (if (`self.Is Menu Enabled`)
      (`self.Input Swipe Right Menu`)
      (else
        (`|MultiGate` false true :!label _label_2
          (:`Out 0`
            (`/Game/ResourceManager/ResourceManager.Try To Accept Law` _resourcemanager _current_law_name)
            (`/Game/UI/Bonanza_HUD.Try To Accept Animation` _bonanza_hud true)
            (goto _label :!via `Reset`))
          (:`Out 1`
            (`/Game/ResourceManager/ResourceManager.Accept Law` _resourcemanager _current_law_name)
            (`self.DisableInput` self)
            (`/Game/UI/Bonanza_HUD.Accept Animation` _bonanza_hud)
            (`KismetSystemLibrary.Delay` 1.0)
            (`self.Display Next Law`)
            (`/Game/UI/Bonanza_HUD.New Law Animation` (`self.Bonanza HUD`))
            (`KismetSystemLibrary.Delay` 0.5)
            (`self.EnableInput` self)))))))

(event `Input Swipe Left Menu`
  (bind _bonanza_hud (`self.Bonanza HUD`))
  (bind _bonanza_hud_2 (`self.Bonanza HUD`))
  ;[1 1 1] Input Swipe Menu
  (`|MultiGate` false true :!label _label_3
    (:`Out 0`
      (`/Game/UI/Bonanza_HUD.Try To Decline Animation` _bonanza_hud true)
      (goto _label_5 :!via `Reset`))
    (:`Out 1`
      (`self.DisableInput` self)
      (`/Game/UI/Bonanza_HUD.Decline Animation` _bonanza_hud)
      (`AudioComponent.FadeOut` (`self.Gameplay Music`) 1.0 0.0 "Linear")
      (`KismetSystemLibrary.Delay` 1.0)
      (`GameplayStatics.OpenLevel` "MainMenu_Level" :!label _label_4))))

(event `Input Swipe Right Menu`
  (bind _bonanza_hud (`self.Bonanza HUD`))
  ;[1 1 1] Input Swipe Menu
  (`|MultiGate` false true :!label _label_5
    (:`Out 0`
      (`/Game/UI/Bonanza_HUD.Try To Accept Animation` _bonanza_hud true)
      (goto _label_3 :!via `Reset`))
    (:`Out 1`
      (`self.DisableInput` self)
      (`/Game/UI/Bonanza_HUD.Accept Animation` _bonanza_hud)
      (`AudioComponent.FadeOut` (`self.Gameplay Music`) 1.0 0.0 "Linear")
      (`KismetSystemLibrary.Delay` 1.0)
      (goto _label_4))))

(fn `Display Next Law`
  (if (not (`self.Is Menu Enabled`))
    (bind (_law_name _law) (`/Game/ResourceManager/ResourceManager.Get Next Law` (`self.ResourceManager`)))
    (bind _output_get (set `self.Current Law Name` _law_name))
    (if (not (== _output_get "None"))
      (`/Game/UI/Bonanza_HUD.Set Law Text` (`self.Bonanza HUD`) "Ustawa" (`.Description_22_2438AFE34C723DC3FEA62FB87FDD3F66` (break `/Game/ResourceManager/LawStructure` _law))))))

(fn `Display Summary`
  (params (`Card Title` :type String) (Text :type String))
  (bind _bonanza_hud (`self.Bonanza HUD`))
  (`/Game/UI/Bonanza_HUD.Toggle Blur` _bonanza_hud true)
  (`/Game/UI/Bonanza_HUD.Set Law Text` _bonanza_hud `Card Title` Text))

(fn `UserConstructionScript`)