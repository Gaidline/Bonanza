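; Main menu player controller that presents starting or quitting the game as a swipeable law card.
; BeginPlay adds the Menu_HUD widget, then briefly disables input while a Polish "Start" card appeals to the mayor and animates in.
; Two MultiGates that reset each other make choices two-step: a first swipe previews, a repeat confirms.
; Confirming right opens Test_Level and confirming left quits, each after locking input and animating.
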(event `self.ReceiveBeginPlay`
  (bind _main_menu_hud (`self.Main Menu HUD`))
  (`|ExecutionSequence`
    (:`then_0`
      (bind _returnvalue (`|CreateWidget` "/Game/UI/Menu_HUD.Menu_HUD_C"))
      (bind _output_get (set `self.Main Menu HUD` _returnvalue))
      (`UserWidget.AddToViewport` _output_get 0))
    (:`then_1`
      (`self.DisableInput` self)
      (`KismetSystemLibrary.Delay` 1.0)
      (`/Game/UI/Menu_HUD.Set Law Text` _main_menu_hud "Start" "Burmistrzu! Miasto Cię potrzebuje!  \n \nPoratujesz?")
      (`/Game/UI/Menu_HUD.New Law Animation` _main_menu_hud)
      (`KismetSystemLibrary.Delay` 0.5)
      (`self.EnableInput` self))))

(event `InputAction|Swipe Left`
  (params (Key :type "Key Structure"))
  (bind _main_menu_hud (`self.Main Menu HUD`))
  (bind _main_menu_hud_2 (`self.Main Menu HUD`))
  ;[1 1 1] Input Swipe
  (:`Pressed`
    (`|MultiGate` false true :!label _label
      (:`Out 0`
        (`/Game/UI/Menu_HUD.Try To Decline Animation` _main_menu_hud_2 true)
        (goto _label_2 :!via `Reset`))
      (:`Out 1`
        (`self.DisableInput` self)
        (`/Game/UI/Menu_HUD.Decline Animation` _main_menu_hud_2)
        (`KismetSystemLibrary.Delay` 1.0)
        (`KismetSystemLibrary.QuitGame` null "Quit")))))

(event `InputAction|Swipe Right`
  (params (Key :type "Key Structure"))
  (bind _main_menu_hud (`self.Main Menu HUD`))
  ;[1 1 1] Input Swipe
  (:`Pressed`
    (`|MultiGate` false true :!label _label_2
      (:`Out 0`
        (`/Game/UI/Menu_HUD.Try To Accept Animation` _main_menu_hud true)
        (goto _label :!via `Reset`))
      (:`Out 1`
        (`self.DisableInput` self)
        (`/Game/UI/Menu_HUD.Accept Animation` _main_menu_hud)
        (`KismetSystemLibrary.Delay` 1.0)
        (`GameplayStatics.OpenLevel` "Test_Level")))))

(fn `UserConstructionScript`)