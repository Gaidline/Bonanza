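; Base building actor that grows and shrinks as a stack of levels, starting with a set number of levels and showing its first tag as text.
; AddNewLevels spawns the next classes from AllBuildingParts as child actor components stacked vertically above Base, tracked by CurrentBuildingParts and CurrentLevelIdx.
; RemoveLevels destroys parts from the top down.
; Event dispatchers signal when the building is completed or has no levels left.
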(event `self.ReceiveBeginPlay`
  (`self.Add New Levels` (`self.Building Startup Levels`))
  (`TextRenderComponent.K2_SetText` (`self.TextRender`) (`KismetTextLibrary.Conv_NameToText` (`|GetArrayItem` (`self.Tags`)))))

(fn `Add New Levels`
  (params (`Num Levels` :type Integer))
  (bind _current_level_idx (`self.Current Level Idx`))
  (bind (_returnvalue_location _returnvalue_rotation) (`KismetMathLibrary.BreakTransform` (`SceneComponent.GetRelativeTransform` (`self.Base`))))
  (for _ (range 1 (+ `Num Levels` 1))
    (if (< _current_level_idx (`KismetArrayLibrary.Array_LastIndex` (`self.All Building Parts`)))
      (bind _result (`/Engine/EditorBlueprintResources/StandardMacros.IncrementInt` _current_level_idx)
        (:`  `
          (bind _returnvalue (`AddComponent|NODE_AddChildActorComponent-0` :`RelativeTransform` (`KismetMathLibrary.MakeTransform` (+ _returnvalue_location (`KismetMathLibrary.MakeVector` 0.0 0.0 (* _result 100.0))) _returnvalue_rotation)))
          (`ChildActorComponent.SetChildActorClass` _returnvalue (`|GetArrayItem` (`self.All Building Parts`) _result))
          (`KismetArrayLibrary.Array_Add` (`self.Current Building Parts`) _returnvalue)))))
  (if (>= (`self.Current Level Idx`) (`KismetArrayLibrary.Array_LastIndex` (`self.All Building Parts`)))
    (`self.Building Completed` self)))

(fn `Remove Levels`
  (params (`Num Levels` :type Integer))
  (bind _current_level_idx (`self.Current Level Idx`))
  (bind _current_building_parts (`self.Current Building Parts`))
  (bind _current_level_idx_2 (`self.Current Level Idx`))
  (bind _output (`|GetArrayItem` _current_building_parts _current_level_idx))
  (for _ (range 1 (+ `Num Levels` 1))
    (if (>= _current_level_idx 0)
      (`/Engine/EditorBlueprintResources/StandardMacros.IsValid` _output
        (:`Is Valid`
          (`ActorComponent.K2_DestroyComponent` _output)
          (`KismetArrayLibrary.Array_Remove` _current_building_parts _current_level_idx_2)
          (`/Engine/EditorBlueprintResources/StandardMacros.DecrementInt` _current_level_idx_2)))))
  (if (< (`self.Current Level Idx`) 0)
    (`self.Building Destroyed` self)))

(fn `UserConstructionScript`)