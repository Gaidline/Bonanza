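; Base building Blueprint that grows and shrinks a building by adding or removing instanced static mesh instances at preset Locations.
; The construction script spawns the startup count, and AddNewInstances adds more while the current index stays within Locations, recording each returned instance index.
; RemoveInstances takes levels off from the current index downward, without trimming the recorded index array.
; Disconnected construction-script logic for syncing an index array to Locations never runs.
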(fn `Add New Instances`
  (params (`Num Instances` :type Integer))
  (locals (`_Instance SM Components` :type "Array of InstancedStaticMeshComponent Object Reference"))
  (bind _current_instance_idx (`self.Current Instance Idx`))
  (for _ (range 1 (+ `Num Instances` 1))
    (if (< _current_instance_idx (`KismetArrayLibrary.Array_LastIndex` (`self.Locations`)))
      (bind _result (`/Engine/EditorBlueprintResources/StandardMacros.IncrementInt` _current_instance_idx)
        (:`  `
          (bind _returnvalue (`InstancedStaticMeshComponent.AddInstance` (`self.InstancedStaticMesh`) (`|GetArrayItem` (`self.Locations`) _result)))
          (`KismetArrayLibrary.Array_Add` (`self.Current Instance Idxs`) _returnvalue))))))

(fn `Remove Instances`
  (params (`Num Levels` :type Integer))
  (bind _current_instance_idx (`self.Current Instance Idx`))
  (for _ (range 1 (+ `Num Levels` 1))
    (if (>= _current_instance_idx 0)
      (`InstancedStaticMeshComponent.RemoveInstance` (`self.InstancedStaticMesh`) (`|GetArrayItem` (`self.Current Instance Idxs`) _current_instance_idx))
      (`/Engine/EditorBlueprintResources/StandardMacros.DecrementInt` _current_instance_idx))))

(fn `UserConstructionScript`
  (`self.Add New Instances` (`self.Num Startup Instances`)))