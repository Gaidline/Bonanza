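; Construction crane actor that swings its top toward a parts depot, a building or a default position, which it faces on BeginPlay.
; The construction script stacks tower meshes from a parts array by startup level count and raises the top to match.
; UpdateCraneRotation finds a horizontal look-at rotation, and a timeline lerps the top to it.
; Trolley movement is computed but its lerp node is disconnected, so only rotation animates.
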(event `self.ReceiveBeginPlay`
  (`self.Rotate Towards Default Position`))

(event `Get Building Part From Depot`
  (`self.Rotate Towards Parts Depot`))

(event `Get Building Part From Building`
  (`self.Rotate Towards Building`))

(event `Update Crane Rotation`
  (params (`Rotate To Relative Position` :type "Vector Structure"))
  (bind _returnvalue (`KismetMathLibrary.MakeVector` 1.0 1.0))
  ;[1 1 1] Update Crane  rotation
  (`|ExecutionSequence`
    (:`then_0`
      (set `self.Target Relative Rotation` (`KismetMathLibrary.FindLookAtRotation` (* _returnvalue (`SceneComponent.RelativeLocation` (`self.Crane Top Center`))) (* `Rotate To Relative Position` _returnvalue)))
      (set `self.Start Relative Rotation` (`SceneComponent.RelativeRotation` (`self.Crane Top Center`)))
      (set `self.Target Relative Location` (- `Rotate To Relative Position` (`SceneComponent.RelativeLocation` (`self.Trolley Center`))))
      (set `self.Start Relative Location` (`SceneComponent.RelativeLocation` (`self.Trolley Center`))))
    (:`then_1`
      (bind (_direction _trolley_position_update _crane_rotation_update) (`Timeline|Crane Rotation` :!via `PlayFromStart`)
        (:`Update`
          (`SceneComponent.K2_SetRelativeRotation` (`self.Crane Top Center`) (`KismetMathLibrary.RLerp` (`self.Start Relative Rotation`) (`self.Target Relative Rotation`) _crane_rotation_update) false false))))))

(fn `Add New Levels`
  (params (`Num Levels` :type Integer))
  (bind _current_level_idx (`self.Current Level Idx`))
  (bind (_returnvalue_location _returnvalue_rotation) (`KismetMathLibrary.BreakTransform` (`SceneComponent.GetRelativeTransform` (`self.Arrow`))))
  (for _ (range 1 (+ `Num Levels` 1))
    (if (< _current_level_idx (`KismetArrayLibrary.Array_LastIndex` (`self.All Crane Parts`)))
      (bind _result (`/Engine/EditorBlueprintResources/StandardMacros.IncrementInt` _current_level_idx)
        (:`  `
          (bind _returnvalue (`AddComponent|NODE_AddStaticMeshComponent-0` :`RelativeTransform` (`KismetMathLibrary.MakeTransform` _returnvalue_location _returnvalue_rotation)))
          (`StaticMeshComponent.SetStaticMesh` _returnvalue (`|GetArrayItem` (`self.All Crane Parts`) _result))
          (`SceneComponent.K2_AddRelativeLocation` _returnvalue (`KismetMathLibrary.MakeVector` 0.0 0.0 (* (.z (`.BoxExtent` (`KismetSystemLibrary.GetComponentBounds` _returnvalue))) (`KismetMathLibrary.Conv_IntToDouble` _result) 2.0)) false false)
          (`KismetArrayLibrary.Array_Add` (`self.Current Crane Parts`))))))
  (`SceneComponent.K2_AddRelativeLocation` (`self.Crane1_TopA`) (`KismetMathLibrary.MakeVector` 0.0 0.0 (* (`self.Current Level Idx`) 120.0)) false false))

(fn `Rotate Towards Building`
  (`self.Update Crane Rotation` (`self.Building Center`)))

(fn `Rotate Towards Default Position`
  (`self.Update Crane Rotation` (`self.Default Position`)))

(fn `Rotate Towards Parts Depot`
  (`self.Update Crane Rotation` (`self.Part Depot Center`)))

(fn `UserConstructionScript`
  (`self.Add New Levels` (`self.Crane Startup Levels`)))